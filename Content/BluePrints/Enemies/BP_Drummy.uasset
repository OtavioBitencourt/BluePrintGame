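; BP_Drummy is an enemy that loses body parts when bullets overlap its hit boxes.
; BeginPlay attaches a spawned melee weapon to a mesh socket, then sets weapon state and health.
; Arm hits hide the left forearm bone; head hits hide the neck bone, ragdoll the mesh and spawn a severed head once.
; Construction strips the inherited camera, spring arm and child actor; the delayed destroy logic is unconnected.
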(event `self.ReceiveBeginPlay`
  (`|ExecutionSequence`
    (:`then_0`
      (bind _returnvalue (`|SpawnActorFromClass` "/Game/BluePrints/Enemies/BP_EnemieWeapon.BP_EnemieWeapon_C" (`KismetMathLibrary.MakeTransform` (0.0 0.0 0.0)) "Undefined" "MultiplyWithRoot" null null))
      (bind _output_get (set `self.MeleeWeapon` _returnvalue))
      (`self.K2_AttachToComponent` _output_get (`self.Mesh`) "OneHandUnequipSocket" "KeepRelative" "KeepRelative" "KeepRelative" true))
    (:`then_1`
      (`self.SetWeaponState` "NewEnumerator1"))
    (:`then_2`
      (set `self.Health` 500.0))))

(event `self.Box.OnComponentBeginOverlap`
  (params (OverlappedComponent :type "PrimitiveComponent Object Reference") (OtherActor :type "Actor Object Reference") (OtherComp :type "PrimitiveComponent Object Reference") (OtherBodyIndex :type Integer) (bFromSweep :type Boolean) (SweepResult :type "HitResult Structure (by ref)"))
  (cast `/Game/BluePrints/Objects/BP_Bullet` OtherActor)
  (`SkinnedMeshComponent.HideBoneByName` (`self.Mesh`) "lowerarm_l" "PBO_None"))

(event `self.BoxHead.OnComponentBeginOverlap`
  (params (OverlappedComponent :type "PrimitiveComponent Object Reference") (OtherActor :type "Actor Object Reference") (OtherComp :type "PrimitiveComponent Object Reference") (OtherBodyIndex :type Integer) (bFromSweep :type Boolean) (SweepResult :type "HitResult Structure (by ref)"))
  (cast `/Game/BluePrints/Objects/BP_Bullet` OtherActor)
  (`|ExecutionSequence`
    (:`then_0`
      (`/Engine/EditorBlueprintResources/StandardMacros.DoOnce` false
        (:`Completed`
          (`|SpawnActorFromClass` "/Game/BluePrints/Enemies/BP_SkeletalHead.BP_SkeletalHead_C" (`self.GetTransform`) "Undefined" "MultiplyWithRoot" null null))))
    (:`then_1`
      (`SkinnedMeshComponent.HideBoneByName` (`self.Mesh`) "neck_01" "PBO_None")
      (`PrimitiveComponent.SetSimulatePhysics` (`self.Mesh`) true))))

(fn `UserConstructionScript`
  (`parent.UserConstructionScript`)
  (`ActorComponent.K2_DestroyComponent` (`self.Camera`))
  (`ActorComponent.K2_DestroyComponent` (`self.SpringArm`))
  (`ActorComponent.K2_DestroyComponent` (`self.ChildActor`))
  (set `self.bSpawnMeleeWeappon` false)
  (set `self.bSpawnRangedWeappon` false))