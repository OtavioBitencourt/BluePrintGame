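; BP_Ammo is an interactable rifle ammo pickup whose prompt shows how many bullets it holds.
; On interact it computes the room left in the player's rifle reserve from BP_Personagem and gives up to that amount via GetAmmo.
; It destroys itself when emptied, otherwise keeps the remainder and refreshes the prompt, or shows an "Ammo full" warning when no room is left.
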(event `self.ReceiveBeginPlay`
  ;[1 1 1] Begin Play
  (`self.SetMessage`))

(event `self.InteractEvent`
  (bind _playerref (`self.PlayerRef`))
  ;[1 1 1] Interact Event
  (`|ExecutionSequence`
    (:`then_0`
      (bind _asbp_personagem (cast `/Game/BluePrints/BP_Personagem` (`GameplayStatics.GetPlayerCharacter` 0)))
      (set `self.PlayerRef` _asbp_personagem))
    (:`then_1`
      (set `self.MaxCollect` (- (`/Game/BluePrints/BP_Personagem.RifleMaxClip` _playerref) (`/Game/BluePrints/BP_Personagem.RifleUloadedAmmo` _playerref))))
    (:`then_2`
      (if (> (`self.MaxCollect`) 0)
        (if (>= (`self.MaxCollect`) (`self.Bullets`))
          (`/Game/BluePrints/BP_Personagem.GetAmmo` (`self.PlayerRef`) (`self.Bullets`))
          (`self.K2_DestroyActor`)
          (else
            (`/Game/BluePrints/BP_Personagem.GetAmmo` (`self.PlayerRef`) (`self.MaxCollect`))
            (set `self.Bullets` (- (`self.Bullets`) (`self.MaxCollect`)))
            (`self.SetMessage`)))
        (else
          (`/Game/BluePrints/BP_Personagem.WarningEvent` (`self.PlayerRef`) "Ammo full" 2.0))))))

(fn `SetMessage`
  (set `self.Message` (`KismetTextLibrary.Conv_StringToText` (`KismetStringLibrary.Concat_StrStr` "Press E to Collect Rifle Ammo(" (`KismetStringLibrary.Conv_IntToString` (`self.Bullets`)) ")"))))

(fn `UserConstructionScript`)