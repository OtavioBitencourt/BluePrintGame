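; Explosive barrel that detonates when a BP_Bullet overlaps its mesh.
; A zero-length multi sphere trace on the Camera channel damages BP_Personagem hits in the surrounding radius.
; It then destroys the mesh, triggers explosion particles and sound, and spawns smoke that a timeline scales before removing it.
; After a short delay, a radial force component fires an impulse.
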(event `self.StaticMesh.OnComponentBeginOverlap`
  (params (OverlappedComponent :type "PrimitiveComponent Object Reference") (OtherActor :type "Actor Object Reference") (OtherComp :type "PrimitiveComponent Object Reference") (OtherBodyIndex :type Integer) (bFromSweep :type Boolean) (SweepResult :type "HitResult Structure (by ref)"))
  (bind _radialforce (`self.RadialForce`))
  (bind _actorlocation (`self.ActorLocation`))
  (if (== (`GameplayStatics.GetObjectClass` OtherActor) "/Game/BluePrints/Objects/BP_Bullet.BP_Bullet_C")
    (`|ExecutionSequence`
      (:`then_0`
        (bind _output_get (set `self.ActorLocation` (`self.K2_GetActorLocation`)))
        (bind _outhits (`KismetSystemLibrary.SphereTraceMulti` :`Start` _output_get :`End` _output_get :`Radius` 300.0 :`TraceChannel` "TraceTypeQuery2" :`bIgnoreSelf` false))
        (for _array_element _outhits
          (bind _asbp_personagem (cast `/Game/BluePrints/BP_Personagem` (`.HitActor` (`GameplayStatics.BreakHitResult` _array_element))))
          (`GameplayStatics.ApplyDamage` _asbp_personagem 100.0 null self)))
      (:`then_1`
        (`ActorComponent.K2_DestroyComponent` (`self.StaticMesh`))
        (`ActorComponent.Activate` (`self.ParticleSystem`) false)
        (`GameplayStatics.SpawnSoundAtLocation` "/Game/StarterContent/Audio/Explosion02.Explosion02" _actorlocation (struct) 1.0 1.0 0.0 null null)
        (bind _returnvalue (`GameplayStatics.SpawnEmitterAtLocation` "/Game/Realistic_Starter_VFX_Pack_Vol2/Particles/Smoke/P_Smoke_B.P_Smoke_B" _actorlocation))
        (bind (_direction _alpha) (`Timeline|SmokeTL` :!via `PlayFromStart`)
          (:`Update`
            (`SceneComponent.SetRelativeScale3D` _returnvalue (`KismetMathLibrary.MakeVector` _alpha _alpha _alpha)))
          (:`Finished`
            (`ActorComponent.K2_DestroyComponent` _returnvalue))))
      (:`then_2`
        (`KismetSystemLibrary.Delay` 0.1)
        (`ActorComponent.Activate` _radialforce false)
        (`RadialForceComponent.FireImpulse` _radialforce)))))

(fn `UserConstructionScript`)