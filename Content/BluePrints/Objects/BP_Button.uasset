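; BP_Button is an interactable button actor that loads the "Survival" level.
; Its capsule overlap sets itself as BP_Personagem's ButtonToRemove reference on entry and clears that reference on exit.
; InteractEvent plays the Musica_Tema sound at the world origin through a DoOnce, then opens the level by name in the same sequence.
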(event `self.Capsule.OnComponentBeginOverlap`
  (params (OverlappedComponent :type "PrimitiveComponent Object Reference") (OtherActor :type "Actor Object Reference") (OtherComp :type "PrimitiveComponent Object Reference") (OtherBodyIndex :type Integer) (bFromSweep :type Boolean) (SweepResult :type "HitResult Structure (by ref)"))
  (bind _asbp_personagem (cast `/Game/BluePrints/BP_Personagem` OtherActor))
  (set `/Game/BluePrints/BP_Personagem.Button_to_Remove` self _asbp_personagem))

(event `self.InteractEvent`
  (`|ExecutionSequence`
    (:`then_0`
      (`/Engine/EditorBlueprintResources/StandardMacros.DoOnce` false
        (:`Completed`
          (`GameplayStatics.PlaySoundAtLocation` "/Game/Assets/Sounds/Musica_Tema.Musica_Tema" (0.0 0.0 0.0) (struct) 1.0 1.0 0.0 null null null null))))
    (:`then_1`
      (`GameplayStatics.OpenLevel` "Survival"))))

(event `self.Capsule.OnComponentEndOverlap`
  (params (OverlappedComponent :type "PrimitiveComponent Object Reference") (OtherActor :type "Actor Object Reference") (OtherComp :type "PrimitiveComponent Object Reference") (OtherBodyIndex :type Integer))
  (bind _asbp_personagem (cast `/Game/BluePrints/BP_Personagem` OtherActor))
  (set `/Game/BluePrints/BP_Personagem.Button_to_Remove` null _asbp_personagem))

(fn `UserConstructionScript`)